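; BP_Gamer is a character Blueprint that sets up walk speed and defines the rule for when sprinting is allowed.
; The construction script copies WalkingSpeed into the movement component's MaxWalkSpeed.
; CanSprint returns true only when the character is not crouching and HealthStats stamina exceeds a fixed minimum.
; The event graph holds only disabled placeholder events, so no sprint or crouch handling appears here.
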(event EventBeginPlay)

(event Collision|EventActorBeginOverlap
  (params (OtherActor :type Actor%20Object%20Reference)))

(event EventTick
  (params (DeltaSeconds :type Float%20%28single-precision%29)))

(fn ConstructionScript
  (Variables|/Script/Engine.CharacterMovementComponent|SetMaxWalkSpeed (Variables|Character|GetCharacterMovement) (Variables|Default|GetWalking%20Speed)))

(fn CanSprint
  (return (and (not (Variables|Default|GetCrouching)) (> (Variables|/Game/Blueprint/Сharacter/Components/HealthStats.HealthStats_C|GetStamina (Variables|Default|GetHealthStats)) 1e+01))))